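; BP_HexTile is a hex grid tile that displays its cube coordinates (Q, R, S) as text.
; On BeginPlay it reads GetCoordinates and fills a combined TextRender label plus separate Q, R and S labels through FormatText.
; The labels are written only at BeginPlay, and the construction script is empty.
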(event `self.ReceiveBeginPlay`
  (bind _returnvalue_q (break `HexCoordinates` (`self.GetCoordinates`)))
  (bind (_returnvalue_q_2 _returnvalue_r _returnvalue_s) (break `HexCoordinates` (`self.GetCoordinates`)))
  (bind (_returnvalue_q_3 _returnvalue_r_2) (break `HexCoordinates` (`self.GetCoordinates`)))
  (bind (_returnvalue_q_4 _returnvalue_r_3 _returnvalue_s_2) (break `HexCoordinates` (`self.GetCoordinates`)))
  (`|ExecutionSequence`
    (:`then_0`
      (`TextRenderComponent.K2_SetText` (`self.TextRender`) (`|FormatText` "q: {q} \nr: {r} \ns: {s}" _returnvalue_q_4 _returnvalue_r_3 _returnvalue_s_2)))
    (:`then_1`
      (`TextRenderComponent.K2_SetText` (`self.S`) (`|FormatText` "s = {s}" _returnvalue_s)))
    (:`then_2`
      (`TextRenderComponent.K2_SetText` (`self.R`) (`|FormatText` "r = {r}" _returnvalue_r_2)))
    (:`then_3`
      (`TextRenderComponent.K2_SetText` (`self.Q`) (`|FormatText` "q = {q}" _returnvalue_q)))))

(fn `UserConstructionScript`)